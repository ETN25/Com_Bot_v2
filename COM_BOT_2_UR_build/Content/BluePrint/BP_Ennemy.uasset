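; BP_Ennemy is an enemy Blueprint that, in the logic shown, only sets up its mesh colors.
; The Construction Script calls BodyColor, which creates and stores dynamic material instances for the mesh's first two material slots.
; The body material takes the BodyColor variable and the logo material takes LaserColor, each through a vector parameter.
; The event graph holds only disabled placeholder events, so it adds no runtime behavior.
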(fn `BodyColor`
  (bind _returnvalue (`PrimitiveComponent.CreateDynamicMaterialInstance` (`self.Mesh`) 0 null "None"))
  (bind _output_get (set `self.Body Material` _returnvalue))
  (`MaterialInstanceDynamic.SetVectorParameterValue` _output_get "BodyColor" (`self.Body_Color`))
  (bind _returnvalue_2 (`PrimitiveComponent.CreateDynamicMaterialInstance` (`self.Mesh`) 1 null "None"))
  (bind _output_get_2 (set `self.Logo_Material` _returnvalue_2))
  (`MaterialInstanceDynamic.SetVectorParameterValue` _output_get_2 "Couleur" (`self.Laser_Color`))
  (return))

(fn `UserConstructionScript`
  (`self.BodyColor`))