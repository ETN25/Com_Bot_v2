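; BP_Gun is a gun Blueprint that fires laser projectiles continuously between its start and stop firing events.
; StartFiring passes through a DoOnce that fires immediately, then sets a looping timer on FireProjectile at a rate derived from ProjectilesPerSeconds.
; FireProjectile spawns an actor at the ProjectilSpawnPoint transform.
; StopFiring clears the timer and resets the DoOnce, which blocks duplicate starts while firing.
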(event `Fire Projectile`
  ;[1 1 1] Tire un Laser
  (`|SpawnActorFromClass` "/Game/BluePrint/BP_Laser.BP_Laser_C" (`SceneComponent.K2_GetComponentToWorld` (`self.Projectil SpawnPoint`)) "Undefined" "OverrideRootScale" null null))

(event `Start Firing`
  ;[1 1 1] Tire en continu
  (`/Engine/EditorBlueprintResources/StandardMacros.DoOnce` false :!label _label
    (:`Completed`
      (`self.Fire Projectile`)
      (`KismetSystemLibrary.K2_SetTimer` null "Fire Projectile" (/ 1.0 (`self.Projectiles per seconds`)) true))))

(event `Stop Firing`
  ;[1 1 1] Stop  tirer
  (`KismetSystemLibrary.K2_ClearTimer` null "Fire Projectile")
  (goto _label :!via `Reset`))

(fn `UserConstructionScript`)